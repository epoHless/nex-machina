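; Wave manager that runs a sequence of enemy waves between two doors, closing the previous one on request and opening the next when all waves are cleared.
; A request resets progress, despawns leftover enemies and activates turrets and humans.
; A looping timer pulls chaser or explosive enemies from object pools and places them at each wave's spawn positions.
; Despawn events track live enemies and advance waves, reactivating turrets each time.
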(event `On Wave Requested`
  (bind _previous_door (`self.Previous Door`))
  (bind _active_enemies (`self.Active Enemies`))
  (`/Engine/EditorBlueprintResources/StandardMacros.IsValid` _previous_door
    (:`Is Valid`
      (`/Game/core/blueprints/generic/level-management/BP_RoomDoor.Close` _previous_door))
    (:`Is Not Valid`
      _))
  (`self.Activate Turrets`)
  (set `self.Wave Index` 0)
  (set `self.Spawn Index` 0)
  (`KismetSystemLibrary.K2_ClearAndInvalidateTimerHandle` (`self.Timer Handle`))
  (for _array_element (`self.Active Enemies`)
    (remove `/Game/core/blueprints/characters/enemies/chaser/BP_PawnChaser.OnObjectDespawned` _array_element (delegate `Pawn Killed`)))
  (`self.Activate Humans`)
  (`/Game/core/blueprints/utilities/BPML_Utilities.Disable All Active Pawn Enemies` _active_enemies (`KismetArrayLibrary.Array_Length` _active_enemies)
    (:`Completed`
      (`KismetArrayLibrary.Array_Clear` (`self.Active Enemies`))
      (bind _output_get (set `self.Current Wave` (`self.Get Current Wave`) :!label _label))
      (bind _output_get_2 (set `self.Time` (`.Delay_8_453C01EC4EFC6F8C12945FA464561842` (break `/Game/core/blueprints/generic/structs/WaveInfo` _output_get))))
      (bind _returnvalue (`KismetSystemLibrary.K2_SetTimerDelegate` (delegate `Spawn Enemy`) _output_get_2 true))
      (set `self.Timer Handle` _returnvalue)
      (add `self.On Waves Cleared` (delegate `On Game Over Event`)))))

(event `On Game Over Event`
  (`KismetSystemLibrary.K2_PauseTimerHandle` (`self.Timer Handle`))
  (`/Game/core/blueprints/generic/level-management/BP_RoomDoor.Open` (`self.Next Door`)))

(event `Spawn Wave`
  (`self.Activate Turrets`)
  (goto _label))

(event `Spawn Enemy`
  (bind _output (`/Game/core/blueprints/characters/enemies/BP_PawnPool.Spawn Object` (`self.Fetch Spawner`)))
  (add `/Game/core/blueprints/characters/enemies/chaser/BP_PawnChaser.OnObjectDespawned` _output (delegate `Pawn Killed`))
  (`self.K2_SetActorLocation` _output (+ (`self.Get Spawn Info Transform`) (0.0 0.0 90.0)) false false)
  (`KismetArrayLibrary.Array_Add` (`self.Active Enemies`) _output)
  (if (`self.Is Wave Spawn Complete`)
    (`KismetSystemLibrary.K2_PauseTimerHandle` (`self.Timer Handle`))
    (else
      (`/Engine/EditorBlueprintResources/StandardMacros.IncrementInt` (`self.Spawn Index`)))))

(event `Pawn Killed`
  (params (Object :type "/Game/core/blueprints/characters/enemies/chaser/BP_PawnChaser Object Reference"))
  (bind _active_enemies (`self.Active Enemies`))
  (remove `/Game/core/blueprints/characters/enemies/chaser/BP_PawnChaser.OnObjectDespawned` Object (delegate `Pawn Killed`))
  (`KismetArrayLibrary.Array_RemoveItem` _active_enemies Object)
  (if (and (<= (`KismetArrayLibrary.Array_Length` _active_enemies) 0) (`self.Is Wave Spawn Complete`))
    (`self.On Wave Cleared`)))

(event `On Wave Cleared`
  (bind (_output_spawninfo _output_delay) (break `/Game/core/blueprints/generic/structs/WaveInfo` (`self.Get Current Wave`)))
  (if (`self.Are All Waves Cleared`)
    (`self.On Waves Cleared`)
    (else
      (set `self.Spawn Index` 0)
      (`/Engine/EditorBlueprintResources/StandardMacros.IncrementInt` (`self.Wave Index`)
        (:`  `
          (set `self.Time` _output_delay)
          (`KismetSystemLibrary.K2_ClearAndInvalidateTimerHandle` (`self.Timer Handle`))
          (`self.Spawn Wave`))))))

(fn `Activate Humans`
  (for _array_element (`self.Humans`)
    (`/Game/core/blueprints/characters/humans/BP_Human.On Request` _array_element)))

(fn `Activate Turrets`
  (for _array_element (`self.Turrets `)
    (`/Game/core/blueprints/characters/enemies/BP_Enemy_Base.Request Object` _array_element)))

(fn `Are All Waves Cleared`
  (returns (Output :type Boolean))
  (return (== (- (`KismetArrayLibrary.Array_Length` (`self.Waves`)) 1) (`self.Wave Index`))))

(fn `Disable Humans`
  (for _array_element (`self.Humans`)
    (`/Game/core/blueprints/characters/humans/BP_Human.Toggle` _array_element "NoCollision" false)))

(fn `Disable Turrets`
  (for _array_element (`self.Turrets `)
    (`PooledObject.Deactivate` _array_element)))

(fn `Fetch Spawner`
  (returns (Pooler :type "/Game/core/blueprints/characters/enemies/BP_PawnPool Object Reference"))
  (bind _current_wave_spawninfo (break `/Game/core/blueprints/generic/structs/WaveInfo` (`self.Current Wave`)))
  (bind (_output_position _output_enemytype) (break `/Game/core/blueprints/generic/structs/SpawnInfo` (`|GetArrayItem` _current_wave_spawninfo (`self.Spawn Index`))))
  (switch `/Game/core/blueprints/generic/misc/enemies/E_EnemyType` _output_enemytype
    (:`NewEnumerator0`
      (return (`/Game/core/blueprints/characters/enemies/BP_EnemyManager.Chaser Pool` (`self.Manager`))))
    (:`NewEnumerator1`
      (return (`/Game/core/blueprints/characters/enemies/BP_EnemyManager.Explosive Pool` (`self.Manager`))))))

(fn `Get Current Wave`
  (returns (Output :type "/Game/core/blueprints/generic/structs/WaveInfo Structure (by ref)"))
  (return (`|GetArrayItem` (`self.Waves`) (`self.Wave Index`))))

(fn `Get Next Wave`
  (returns (Output :type "/Game/core/blueprints/generic/structs/WaveInfo Structure (by ref)"))
  (bind _waves (`self.Waves`))
  (return (`|GetArrayItem` _waves (+ (`KismetArrayLibrary.Array_Find` _waves (`self.Current Wave`)) 1))))

(fn `Get Spawn Info Transform`
  (returns (Transform :type "Vector Structure (by ref)"))
  (bind _output_spawninfo (break `/Game/core/blueprints/generic/structs/WaveInfo` (`self.Get Current Wave`)))
  (bind _output_position (break `/Game/core/blueprints/generic/structs/SpawnInfo` (`|GetArrayItem` _output_spawninfo (`self.Spawn Index`))))
  (return _output_position))

(fn `Is Wave Spawn Complete`
  (returns (ReturnValue :type Boolean))
  (bind _output_spawninfo (break `/Game/core/blueprints/generic/structs/WaveInfo` (`self.Get Current Wave`)))
  (return (>= (`self.Spawn Index`) (- (`KismetArrayLibrary.Array_Length` _output_spawninfo) 1))))

(fn `UserConstructionScript`)