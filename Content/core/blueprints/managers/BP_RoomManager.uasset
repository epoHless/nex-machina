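; Room manager Blueprint that reports a room's progress through two events, room advance and room cleared.
; On BeginPlay it binds to its WaveManager's waves-cleared event and its Spawn's spawner-triggered event.
; A triggered spawner broadcasts room advance, while cleared waves make the WaveManager disable turrets and humans before the room-cleared broadcast.
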(event `self.ReceiveBeginPlay`
  (add `/Game/core/blueprints/managers/BP_WaveManager.On Waves Cleared` (`self.Wave Manager`) (delegate `Complete Room`))
  (add `/Game/core/blueprints/generic/level-management/BP_RoomSpawn.OnSpawnerTriggered` (`self.Spawn`) (delegate `On Spawner Triggered`)))

(event `On Spawner Triggered`
  (`self.On Room Advance`))

(event `Complete Room`
  (bind _wave_manager (`self.Wave Manager`))
  (`/Game/core/blueprints/managers/BP_WaveManager.Disable Turrets` _wave_manager)
  (`/Game/core/blueprints/managers/BP_WaveManager.Disable Humans` _wave_manager)
  (`self.On Room Cleared`))

(fn `UserConstructionScript`)