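; BP_Bullet is a reusable, pool-style projectile that damages what it overlaps.
; When requested, it launches via ProjectileMovement along the given direction scaled by Speed, in local space, and shows its particle.
; On collision overlap it calls TakeDamage on the other actor's HealthComponent, if present, then deactivates regardless of what it hit.
; Deactivation hides the particle.
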(event `self.OnObjectRequest`
  (params (Direction :type "Vector Structure"))
  (`ProjectileMovementComponent.SetVelocityInLocalSpace` (`self.ProjectileMovement`) (* Direction (`self.Speed`)))
  (`SceneComponent.SetVisibility` (`self.Particle`) true false))

(event `self.Collision.OnComponentBeginOverlap`
  (params (OverlappedComponent :type "PrimitiveComponent Object Reference") (OtherActor :type "Actor Object Reference") (OtherComp :type "PrimitiveComponent Object Reference") (OtherBodyIndex :type Integer) (bFromSweep :type Boolean) (SweepResult :type "HitResult Structure (by ref)"))
  (bind _returnvalue (`self.GetComponentByClass` OtherActor "/Script/NexCore.HealthComponent"))
  (`|ExecutionSequence`
    (:`then_0`
      (if (`KismetSystemLibrary.IsValid` _returnvalue)
        (`HealthComponent.TakeDamage` _returnvalue)))
    (:`then_1`
      (`self.Deactivate`))))

(event `self.OnObjectDeactivated`
  (`SceneComponent.SetVisibility` (`self.Particle`) false false))

(fn `UserConstructionScript`)