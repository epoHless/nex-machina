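; Player weapon Blueprint that rotates to a requested direction and fires pooled bullets, with muzzle flash and sound.
; BeginPlay loads the Rifle row from DT_Weapons as the loadout, which InitializeWeapon uses to set fire rate and fill bullet and particle pools.
; Shoot requests wait out the fire rate, then fire along each indexed muzzle's rotation from the actor's location.
; Bullet despawns place pooled hit particles at the bullet's location.
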(event `self.ReceiveBeginPlay`
  (bind _returnvalue (`|GetDataTableRow` "/Game/core/blueprints/generic/weapons/data/DT_Weapons.DT_Weapons" "Rifle")
    (:`then`
      (set `self.Equipped Loadout` _returnvalue))))

(event `Initialize Weapon`
  (`self.Initialize`)
  (`FXSystemComponent.SetFloatParameter` (`self.MuzzleFlash`) "Delay" (`self.Fire Rate`))
  (add `/Game/core/blueprints/generic/weapons/BP_ShootingComponent.OnDespawn` (`self.Bullet Pool`) (delegate `CustomEvent`))
  (set `self.Muzzles` (`|MakeArray` (`self.Muzzle1`) (`self.Muzzle2`) (`self.Muzzle3`))))

(event `CustomEvent`
  (params (Object :type "PooledObject Object Reference"))
  (bind _returnvalue (`ObjectPool.SpawnPooledObject` (`self.Particle Pool`)))
  (`self.K2_SetActorLocation` _returnvalue (`self.K2_GetActorLocation` Object) false false))

(event `self.On Shoot Request`
  (params (`X Value` :type "Float (double-precision)") (`Y Value` :type "Float (double-precision)") (Rotation :type Boolean))
  (bind _returnvalue (`self.K2_GetActorLocation`))
  (if (`self.Rotate In Direction` `X Value` `Y Value` Rotation)
    (`KismetSystemLibrary.Delay` (`self.Fire Rate`))
    (for _index (range (+ (`self.Muzzle Count`) 1))
      (`SceneComponent.K2_SetWorldLocationAndRotation` (`self.Muzzle`) _returnvalue (`SceneComponent.K2_GetComponentRotation` (`|GetArrayItem` (`self.Muzzles`) _index)) false false)
      (`self.Shoot`)
      (`ActorComponent.Activate` (`self.MuzzleFlash`) true)
      (`GameplayStatics.PlaySoundAtLocation` "/Game/core/art/sounds/SFX_Player_Shot.SFX_Player_Shot" _returnvalue (struct) 0.4 1.0 0.0 "/Game/core/art/sounds/attenuation/NewSoundAttenuation_Turrets.NewSoundAttenuation_Turrets" null null null))
    (else
      (`ActorComponent.Deactivate` (`self.MuzzleFlash`)))))

(fn `Initialize`
  (bind (_equipped_loadout_firerate _equipped_loadout_bullet _equipped_loadout_hitparticle) (break `/Game/core/blueprints/generic/weapons/data/WeaponData` (`self.Equipped Loadout`)))
  (set `self.Fire Rate` _equipped_loadout_firerate)
  (set `ObjectPool.PooledObjectSubclass` _equipped_loadout_hitparticle (`self.Particle Pool`))
  (set `ObjectPool.PooledObjectSubclass` _equipped_loadout_bullet (`self.Bullet Pool`))
  (set `self.Hit Type` _equipped_loadout_hitparticle)
  (`ObjectPool.InstantiatePoolableActors` (`self.Particle Pool`))
  (`ObjectPool.InstantiatePoolableActors` (`self.Bullet Pool`)))

(fn `UserConstructionScript`
  (`parent.UserConstructionScript`))