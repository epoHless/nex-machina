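; BP_Sword is a melee weapon that swings on demand and deals 1 damage to overlapped actors with a BP_EnemyHealthComponent.
; Swing is gated by CanSwing and plays a timeline that yaws the sword mesh through a linear half-turn, then re-arms.
; Toggle shows both meshes and enables overlap events during the swing, reversing both afterward, though both calls pass NoCollision to the hit component.
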(event `Swing`
  (if (`self.Can Swing`)
    (`self.Toggle` true)
    (set `self.Can Swing` false)
    (bind (_direction _value) (`Timeline|Swing Sword` :!via `PlayFromStart`)
      (:`Update`
        (`SceneComponent.K2_SetRelativeRotation` (`self.SM_Wep_Sword_01`) (`KismetMathLibrary.MakeRotator` -90.0 0.0 (`|EaseFunction` "Linear" _value 0.0 180.0)) false false))
      (:`Finished`
        (set `self.Can Swing` true)
        (`self.Toggle` false)))))

(event `self.Collision.OnComponentBeginOverlap`
  (params (OverlappedComponent :type "PrimitiveComponent Object Reference") (OtherActor :type "Actor Object Reference") (OtherComp :type "PrimitiveComponent Object Reference") (OtherBodyIndex :type Integer) (bFromSweep :type Boolean) (SweepResult :type "HitResult Structure (by ref)"))
  (bind _returnvalue (`self.GetComponentByClass` OtherActor "/Game/core/blueprints/generic/health-component/BP_EnemyHealthComponent.BP_EnemyHealthComponent_C"))
  (`/Engine/EditorBlueprintResources/StandardMacros.IsValid` _returnvalue
    (:`Is Valid`
      (`HealthComponent.TakeDamage` _returnvalue 1))))

(fn `Toggle`
  (params (Toggle :type Boolean) (Collision :type "ECollisionEnabled Enum" :default "NoCollision"))
  (bind _collision (`self.Collision`))
  (`SceneComponent.SetVisibility` (`self.SM_Wep_Sword_01`) Toggle Toggle)
  (`SceneComponent.SetVisibility` (`self.SM_Wep_Sword_02`) Toggle Toggle)
  (`PrimitiveComponent.SetCollisionEnabled` _collision Collision)
  (set `PrimitiveComponent.bGenerateOverlapEvents` Toggle _collision))

(fn `UserConstructionScript`)