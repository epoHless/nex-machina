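; BP_Shooter is a generic weapon actor that fires pooled bullets from its muzzle in response to directional input.
; Shoot requests with non-zero input optionally rotate the actor, then fire after a FireRate Delay that throttles repeated requests; zero input deactivates the muzzle flash.
; Bullet despawns place pooled hit particles at the bullet's location.
; A setup function configures fire rate, bullet pool size and lifetime.
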(event `On Shoot Request`
  (params (`X Value` :type "Float (double-precision)") (`Y Value` :type "Float (double-precision)") (Rotation :type Boolean))
  (if (`self.Rotate In Direction` `X Value` `Y Value` Rotation)
    (`KismetSystemLibrary.Delay` (`self.Fire Rate`))
    (`self.Shoot`)
    (`ActorComponent.Activate` (`self.MuzzleFlash`) true)
    (else
      (`ActorComponent.Deactivate` (`self.MuzzleFlash`)))))

(event `self.ReceiveBeginPlay`
  (set `/Game/core/blueprints/generic/weapons/BP_ShootingComponent.Pooled Object Type` (`self.Bullet Type`) (`self.Bullet Pool`))
  (`FXSystemComponent.SetFloatParameter` (`self.MuzzleFlash`) "Delay" (`self.Fire Rate`))
  (add `/Game/core/blueprints/generic/weapons/BP_ShootingComponent.OnDespawn` (`self.Bullet Pool`) (delegate `Spawn Hit Particle`)))

(event `Spawn Hit Particle`
  (params (Object :type "PooledObject Object Reference"))
  (bind _returnvalue (`ObjectPool.SpawnPooledObject` (`self.Particle Pool`)))
  (`self.K2_SetActorLocation` _returnvalue (`self.K2_GetActorLocation` Object) false false))

(fn `Rotate In Direction`
  (params (`X Value` :type "Float (double-precision)") (`Y Value` :type "Float (single-precision)") (Rotation :type Boolean))
  (returns (`Should Shoot` :type Boolean))
  (bind _returnvalue (`KismetMathLibrary.MakeVector` `X Value` `Y Value`))
  (if Rotation
    (`self.K2_SetActorRotation` (`KismetMathLibrary.Conv_VectorToRotator` _returnvalue)))
  (return (> (`KismetMathLibrary.VSize` _returnvalue) 0.0)))

(fn `Setup Shooting Component`
  (params (`Fire Rate` :type "Float (double-precision)") (`Pool Size` :type Integer) (`Life Time` :type "Float (double-precision)"))
  (bind _bullet_pool (`self.Bullet Pool`))
  (set `self.Fire Rate` `Fire Rate`)
  (set `ObjectPool.PoolSize` `Pool Size` _bullet_pool)
  (set `ObjectPool.PooledObjectLifeTime` `Life Time` _bullet_pool))

(fn `Shoot`
  (bind _muzzle (`self.Muzzle`))
  (bind _returnvalue (`ObjectPool.SpawnPooledObject` (`self.Bullet Pool`)))
  (`self.K2_SetActorLocationAndRotation` _returnvalue (`SceneComponent.K2_GetComponentLocation` _muzzle) (`SceneComponent.K2_GetComponentRotation` _muzzle) false false))

(fn `UserConstructionScript`)