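; BP_Gun is a generic gun Blueprint that fires pooled objects from its muzzle.
; Shoot takes an object from BPShootingComponent's pool and moves it to the Muzzle's world location and rotation.
; A setup function passes pool size and object lifetime to that component and stores a fire rate, which Shoot itself does not use.
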(fn `Setup Shooting Component`
  (params (`Fire Rate` :type "Float (double-precision)") (`Pool Size` :type Integer) (`Life Time` :type "Float (double-precision)"))
  (bind _bp_shootingcomponent (`self.BP_ShootingComponent`))
  (set `self.Fire Rate` `Fire Rate`)
  (set `ObjectPool.PoolSize` `Pool Size` _bp_shootingcomponent)
  (set `ObjectPool.PooledObjectLifeTime` `Life Time` _bp_shootingcomponent))

(fn `Shoot`
  (bind _muzzle (`self.Muzzle`))
  (bind _returnvalue (`ObjectPool.SpawnPooledObject` (`self.BP_ShootingComponent`)))
  (`self.K2_SetActorLocationAndRotation` _returnvalue (`SceneComponent.K2_GetComponentLocation` _muzzle) (`SceneComponent.K2_GetComponentRotation` _muzzle) false false))

(fn `UserConstructionScript`)