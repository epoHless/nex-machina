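; Player dash component that launches a character horizontally and runs a cooldown afterwards.
; The Dash event scales the X and Y inputs by LaunchForce, adds that velocity through LaunchCharacter without overriding current velocity, and clears Enabled.
; Tick counts the cooldown down while disabled, then resets it and sets Enabled again.
; Dash itself does not check Enabled.
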(event `self.ReceiveBeginPlay`
  (`self.Set Cooldown Time`))

(event `Dash`
  (params (Player :type "NexCharacter Object Reference") (X :type "Float (double-precision)") (Y :type "Float (double-precision)"))
  (`Character.LaunchCharacter` Player (`self.Set Launch Velocity` X Y) false false)
  (set `self.Enabled` false))

(event `self.ReceiveTick`
  (params (DeltaSeconds :type "Float (single-precision)"))
  (if (not (`self.Enabled`))
    (bind _output_get (set `self.Current Cooldown` (- (`self.Current Cooldown`) (`GameplayStatics.GetWorldDeltaSeconds`))))
    (if (<= _output_get 0.0)
      (`self.Set Cooldown Time`)
      (set `self.Enabled` true))))

(fn `Set Cooldown Time`
  (set `self.Current Cooldown` (`self.Cooldown Time`)))

(fn `Set Launch Velocity`
  (params (A_X :type "Float (single-precision)") (A_Y :type "Float (single-precision)"))
  (returns (ReturnValue :type "Vector Structure"))
  (return (* (`KismetMathLibrary.MakeVector` A_X A_Y) (`KismetMathLibrary.Conv_DoubleToVector` (`self.Launch Force`)))))