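; BP_Ship is a ship actor that moves back and forth on a looping timeline, starting at BeginPlay.
; The Float timeline drives a linear blend from the stored start location toward the End offset added to the actor's current location, re-read on each update.
; When the timeline finishes, it checks its direction and restarts the opposite way, repeating indefinitely.
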(event `self.ReceiveBeginPlay`
  (bind _output_get (set `self.Start` (`self.K2_GetActorLocation`)))
  (bind (_direction _value) (`Timeline|Float` :!via `PlayFromStart` :!label _label)
    (:`Update`
      (`self.K2_SetActorLocation` (`|EaseFunction` "Linear" _value _output_get (+ (`self.End`) (`self.K2_GetActorLocation`)))))
    (:`Finished`
      (switch `ETimelineDirection` _direction
        (:`Forward`
          (`self.Reverse`))
        (:`Backward`
          (`self.Play`))))))

(event `Play`
  (goto _label :!via `PlayFromStart`))

(event `Reverse`
  (goto _label :!via `ReverseFromEnd`))

(fn `UserConstructionScript`)