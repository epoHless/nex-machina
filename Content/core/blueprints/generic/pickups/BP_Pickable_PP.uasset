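; Pooled power-up pickup that gives the player a randomly selected power-up.
; When requested, it sets its power-up and mesh through separate GetRandomPowerUp calls and enables overlap events on its sphere.
; On pickup it executes the power-up on the player and deactivates, and deactivation turns overlap events off until the next request.
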(event `self.OnObjectRequest`
  (params (Direction :type "Vector Structure"))
  (`self.Setup Power Up`))

(event `self.OnPickup`
  (params (Player :type "NexCharacter Object Reference"))
  (`PowerUp.Execute` (`self.GetPowerUp`) Player)
  (`self.Deactivate`))

(event `self.OnObjectDeactivated`
  (`self.Toggle Overlap` false))

(fn `Setup Power Up`
  (bind (_output_powerup _output_mesh) (break `/Game/core/blueprints/generic/pickups/power-ups/data/STR_PPData` (`/Game/core/blueprints/generic/pickups/power-ups/FL_PowerUps.GetRandomPowerUp`)))
  (set `self.PowerUp` _output_powerup)
  (`StaticMeshComponent.SetStaticMesh` (`self.Mesh`) _output_mesh)
  (`self.Toggle Overlap` true))

(fn `Toggle Overlap`
  (params (Toggle :type Boolean))
  (set `PrimitiveComponent.bGenerateOverlapEvents` Toggle (`self.SphereComponent`)))

(fn `UserConstructionScript`)