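; BP_PPProcessor is a power-up processor on BP_Player that strips the player's power-ups when a life is lost.
; On BeginPlay it casts its owner to BP_Player, caches it and binds to the HealthComponent's OnLifeLost event.
; When that event fires, it calls OnRemove on each entry in its PowerUps array, passing the player, then clears the array.
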(event `self.ReceiveBeginPlay`
  (bind _asbp_player (cast `/Game/core/blueprints/characters/player/BP_Player` (`self.GetOwner`)))
  (bind _output_get (set `self.Player` _asbp_player))
  (add `/Game/core/blueprints/generic/health-component/BP_PlayerHealthComponent.On Life Lost` (`/Game/core/blueprints/characters/player/BP_Player.Health Component` _output_get) (delegate `On Life Lost`)))

(event `On Life Lost`
  (params (`Current Health` :type Integer))
  (for _array_element (`self.PowerUps`)
    (`PowerUp.OnRemove` _array_element (`self.Player`)))
  (`KismetArrayLibrary.Array_Clear` (`self.PowerUps`)))