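; Wandering human pawn that the player collects for score by touching it, while enemy contact removes it without awarding points.
; On request it becomes visible and collidable, scales in through a timeline, then endlessly chains AI moves to random nearby navigable points.
; Toggle switches collision, overlaps and mesh visibility instead of spawning or destroying the actor, stopping movement when switched off.
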(event `On Request`
  (`self.Toggle` "QueryAndPhysics" true)
  (bind (_direction _value) (`Timeline|Timeline_0` :!via `PlayFromStart`)
    (:`Update`
      (`self.SetActorScale3D` (`KismetMathLibrary.Conv_DoubleToVector` _value)))
    (:`Finished`
      (`|AIMoveTo` null (`NavigationSystemV1.K2_GetRandomLocationInNavigableRadius` (`self.K2_GetActorLocation`) 200.0 null null) null :!label _label
        (:`OnSuccess`
          _)
        (:`OnFail`
          _))
      (`self.Restart`))))

(event `Restart`
  (goto _label))

(event `On Despawn`
  (`ScoreSubsystem.AssignScore` (subsystem `ScoreSubsystem`) 200.0 0.0)
  (`self.Toggle` "NoCollision"))

(event `self.Collision.OnComponentBeginOverlap`
  (params (OverlappedComponent :type "PrimitiveComponent Object Reference") (OtherActor :type "Actor Object Reference") (OtherComp :type "PrimitiveComponent Object Reference") (OtherBodyIndex :type Integer) (bFromSweep :type Boolean) (SweepResult :type "HitResult Structure (by ref)"))
  (cast `EnemyPawn` OtherActor
    (:`then`
      (`self.Toggle` "NoCollision"))
    (:`CastFailed`
      (cast `/Game/core/blueprints/characters/player/BP_Player` OtherActor)
      (`self.On Despawn`))))

(fn `Toggle`
  (params (Collision :type "ECollisionEnabled Enum" :default "NoCollision") (Toggle :type Boolean))
  (bind _collision (`self.Collision`))
  (`PrimitiveComponent.SetCollisionEnabled` _collision Collision)
  (set `PrimitiveComponent.bGenerateOverlapEvents` Toggle _collision)
  (`SceneComponent.SetVisibility` (`self.Mesh`) Toggle false)
  (if (not Toggle)
    (`NavMovementComponent.StopActiveMovement` (`self.FloatingPawnMovement`))))

(fn `UserConstructionScript`)