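; Player component that manages special attacks, creating an object from each configured class at BeginPlay and selecting the first as current.
; Execute runs the current attack only if enabled, then disables it and starts a cooldown timer.
; The timer passes ReloadTime as both time and initial delay, so re-enabling takes twice ReloadTime.
; A dispatcher broadcasts the attack on use and on reset.
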(event `self.ReceiveBeginPlay`
  (for _array_element (`self.Special Attacks`)
    (bind _returnvalue (`|GenericCreateObject` _array_element))
    (`KismetArrayLibrary.Array_Add` (`self.Special Attacks Param`) _returnvalue))
  (set `self.Current Special Attack` (`|GetArrayItem` (`self.Special Attacks Param`))))

(event `On Attack Executed`
  (bind _current_special_attack (`self.Current Special Attack`))
  (bind _reload_time (`/Game/core/blueprints/characters/player/special/attacks/Exec_SpecialAttack.Reload Time` (`self.Current Special Attack`)))
  (`KismetSystemLibrary.K2_SetTimerDelegate` (delegate `Reset`) _reload_time false _reload_time)
  (set `/Game/core/blueprints/characters/player/special/attacks/Exec_SpecialAttack.Enabled` false _current_special_attack)
  (`/Game/core/blueprints/characters/player/special/attacks/Exec_SpecialAttack.Execute` _current_special_attack self))

(event `Reset`
  (bind _current_special_attack (`self.Current Special Attack`))
  (set `/Game/core/blueprints/characters/player/special/attacks/Exec_SpecialAttack.Enabled` true _current_special_attack)
  (`self.On Special Attack Called` _current_special_attack))

(fn `Execute`
  (if (`/Game/core/blueprints/characters/player/special/attacks/Exec_SpecialAttack.Enabled` (`self.Current Special Attack`))
    (`self.On Attack Executed`)
    (`self.On Special Attack Called` (`self.Current Special Attack`))))