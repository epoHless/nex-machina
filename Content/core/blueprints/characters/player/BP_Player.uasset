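; BP_Player is the player character Blueprint, routing input to shooting, dashing and special attacks.
; On BeginPlay it caches the child-actor gun as a BP_Shooter and spawns socket gun and shield actors attached to the mesh.
; Rotation axes feed the gun's shoot requests, while dashes notify the HealthComponent, which also holds the toggleable vulnerability flag.
; Capsule overlaps trigger pickups through the Pickable interface.
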(event `self.ReceiveBeginPlay`
  (`self.Setup Gun`))

(event `InputAction|Special Attack`
  (params (Key :type "Key Structure"))
  (:`Pressed`
    (`/Game/core/blueprints/characters/player/special/BP_SpecialAttackComponent.Execute` (`self.Special Attacks Component`))))

(event `InputAxis|X Rotation`
  (params (AxisValue :type "Float (single-precision)"))
  (`/Game/core/blueprints/generic/weapons/BP_Shooter.On Shoot Request` (`self.Player Gun`) AxisValue (stale `InputAxis|Y Rotation` AxisValue) true :!label _label))

(event `InputAction|Dash`
  (params (Key :type "Key Structure"))
  (bind _dash_component (`self.Dash Component`))
  (:`Pressed`
    (if (`/Game/core/blueprints/generic/player-components/BP_DashComponent.Enabled` _dash_component)
      (`/Game/core/blueprints/generic/player-components/BP_DashComponent.Dash` _dash_component self (`self.GetInputAxisValue`) (`self.GetInputAxisValue`))
      (`/Game/core/blueprints/generic/health-component/BP_PlayerHealthComponent.On Dash` (`self.Health Component`)))))

(event `InputAxis|Y Rotation`
  (params (AxisValue :type "Float (single-precision)"))
  (goto _label))

(event `self.CapsuleComponent.OnComponentBeginOverlap`
  (params (OverlappedComponent :type "PrimitiveComponent Object Reference") (OtherActor :type "Actor Object Reference") (OtherComp :type "PrimitiveComponent Object Reference") (OtherBodyIndex :type Integer) (bFromSweep :type Boolean) (SweepResult :type "HitResult Structure (by ref)"))
  (if (`KismetSystemLibrary.DoesImplementInterface` OtherActor "/Script/NexCore.Pickable")
    (message `Pickable.OnPickup` OtherActor self)))

(fn `Setup Gun`
  (bind _asbp_shooter (cast `/Game/core/blueprints/generic/weapons/BP_Shooter` (`ChildActorComponent.ChildActor` (`self.Gun`))))
  (set `self.Player Gun` _asbp_shooter)
  (bind _returnvalue (`|SpawnActorFromClass` "/Game/core/blueprints/characters/player/BP_SocketGun.BP_SocketGun_C" (`SceneComponent.GetSocketTransform` (`self.Mesh`) "Hand_r_Weapone_Socket" "RTS_World") "Undefined" "OverrideRootScale" null null))
  (`self.K2_AttachToComponent` _returnvalue (`self.Mesh`) "Hand_r_Weapone_Socket" "SnapToTarget" "SnapToTarget" "SnapToTarget" true)
  (bind _returnvalue_2 (`|SpawnActorFromClass` "/Game/core/blueprints/generic/pickups/power-ups/vfx/BP_Shield.BP_Shield_C" (`SceneComponent.GetSocketTransform` (`self.Mesh`) "Hand_r_Weapone_Socket" "RTS_World") "Undefined" "OverrideRootScale" null null))
  (bind _output_get (set `self.Shield` _returnvalue_2))
  (`self.K2_AttachToComponent` _output_get (`self.Mesh`) "ShieldSocket" "SnapToTarget" "SnapToTarget" "SnapToTarget" true))

(fn `Toggle Invulnerable`
  (params (`Is Vulnerable` :type Boolean))
  (set `/Game/core/blueprints/generic/health-component/BP_PlayerHealthComponent.Is Vulnerable` `Is Vulnerable` (`self.Health Component`)))

(fn `UserConstructionScript`)