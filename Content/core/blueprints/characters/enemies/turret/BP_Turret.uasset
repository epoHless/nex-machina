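; BP_Turret is an enemy turret that shoots and turns toward the player while its detection sphere is overlapped.
; A looping timer at the child-actor shooter's fire rate starts paused, unpauses on player overlap or RequestObject, and pauses on end overlap or death.
; Each tick fires along the current forward vector, then a timeline eases yaw toward the player, so aim trails the target.
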(event `self.ReceiveBeginPlay`
  (`parent.ReceiveBeginPlay`)
  (bind _asbp_shooter (cast `/Game/core/blueprints/generic/weapons/BP_Shooter` (`ChildActorComponent.ChildActor` (`self.Shooter Component`))))
  (set `self.Shooter` _asbp_shooter)
  (`SphereComponent.SetSphereRadius` (`self.Player Detection`) (`self.Detection Radius`) true)
  (bind _returnvalue (`KismetSystemLibrary.K2_SetTimerDelegate` (delegate `Shoot`) (`/Game/core/blueprints/generic/weapons/BP_Shooter.Fire Rate` (`self.Shooter`)) true))
  (bind _output_get (set `self.Timer Handle` _returnvalue))
  (`KismetSystemLibrary.K2_PauseTimerHandle` _output_get))

(event `Shoot`
  (bind (_returnvalue_x _returnvalue_y) (`KismetMathLibrary.BreakVector` (`self.GetActorForwardVector`)))
  (bind (_returnvalue_roll _returnvalue_pitch _returnvalue_yaw) (`KismetMathLibrary.BreakRotator` (`self.K2_GetActorRotation`)))
  (`/Game/core/blueprints/generic/weapons/BP_Shooter.On Shoot Request` (`self.Shooter`) _returnvalue_x _returnvalue_y false)
  (bind (_direction _value) (`Timeline|Rotation` :!via `PlayFromStart`)
    (:`Update`
      (`self.K2_SetActorRotation` (`KismetMathLibrary.MakeRotator` 0.0 0.0 (`|EaseFunction` "Linear" _value _returnvalue_yaw (`self.Set Rotation`)))))))

(event `self.Player Detection.OnComponentBeginOverlap`
  (params (OverlappedComponent :type "PrimitiveComponent Object Reference") (OtherActor :type "Actor Object Reference") (OtherComp :type "PrimitiveComponent Object Reference") (OtherBodyIndex :type Integer) (bFromSweep :type Boolean) (SweepResult :type "HitResult Structure (by ref)"))
  (bind _asbp_player (cast `/Game/core/blueprints/characters/player/BP_Player` OtherActor))
  (if (not (`KismetSystemLibrary.IsValid` (`self.Player`)))
    (set `self.Player` _asbp_player))
  (`KismetSystemLibrary.K2_UnPauseTimerHandle` (`self.Timer Handle`)))

(event `self.Player Detection.OnComponentEndOverlap`
  (params (OverlappedComponent :type "PrimitiveComponent Object Reference") (OtherActor :type "Actor Object Reference") (OtherComp :type "PrimitiveComponent Object Reference") (OtherBodyIndex :type Integer))
  (`KismetSystemLibrary.K2_PauseTimerHandle` (`self.Timer Handle`)))

(event `self.On Death`
  (`parent.On Death`)
  (`KismetSystemLibrary.K2_PauseTimerHandle` (`self.Timer Handle`)))

(event `self.Request Object`
  (`KismetSystemLibrary.K2_UnPauseTimerHandle` (`self.Timer Handle`)))

(fn `Set Rotation`
  (returns (ReturnValue_Yaw :type "Float (single-precision)"))
  (bind (_returnvalue_roll _returnvalue_pitch _returnvalue_yaw) (`KismetMathLibrary.BreakRotator` (`KismetMathLibrary.FindLookAtRotation` (`self.K2_GetActorLocation`) (`self.K2_GetActorLocation` (`self.Player`)))))
  (return _returnvalue_yaw))

(fn `UserConstructionScript`)