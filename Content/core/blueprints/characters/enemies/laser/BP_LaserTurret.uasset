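; Laser turret enemy that slides back and forth while tracing a laser for the player, built on a parent with request/deactivate events.
; RequestObject enables Tick and starts a curve-driven timeline that ping-pongs the capsule between start and offset end positions with easing.
; Tick line-traces at fixed height along the mesh's right vector, calling TakeDamage on a hit player's health component.
; Death or deactivation stops movement and Tick.
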(event `self.ReceiveBeginPlay`
  (bind _returnvalue (`self.K2_GetActorLocation`))
  (bind _movement (`self.Movement`))
  (set `self.Enabled` false)
  (`FXSystemComponent.SetVectorParameter` (`self.Niagara`) "End Position" (* (`self.GetActorForwardVector`) (`self.Laser Distance`)))
  (`parent.ReceiveBeginPlay`)
  (set `self.Start Pos` _returnvalue)
  (set `self.End Pos` (+ (`self.End Pos`) _returnvalue))
  (`TimelineComponent.SetTimelineLength` _movement (`.MaxTime` (`CurveBase.GetTimeRange` (`self.Movement Curve`))))
  (`TimelineComponent.SetFloatCurve` _movement (`self.Movement Curve`) "Value"))

(event `self.ReceiveTick`
  (params (DeltaSeconds :type "Float (single-precision)"))
  (bind _returnvalue (`self.K2_GetActorLocation`))
  (bind (_x _y) (`KismetMathLibrary.BreakVector3f` _returnvalue))
  (bind (_end_position_x _end_position_y) (`KismetMathLibrary.BreakVector` (`self.Get Laser End Position` _returnvalue (`SceneComponent.GetRightVector` (`self.Mesh`)))))
  (bind _outhit (`KismetSystemLibrary.LineTraceSingle` :`Start` (`KismetMathLibrary.MakeVector` _x _y 80.0) :`End` (`KismetMathLibrary.MakeVector` _end_position_x _end_position_y 80.0) :`TraceChannel` "TraceTypeQuery2" :`DrawDebugType` "ForOneFrame"))
  (bind _asbp_player (cast `/Game/core/blueprints/characters/player/BP_Player` (`.HitActor` (`GameplayStatics.BreakHitResult` _outhit))))
  (`HealthComponent.TakeDamage` (`self.GetComponentByClass` (`.HitActor` (`GameplayStatics.BreakHitResult` _outhit)) "/Script/NexCore.HealthComponent") 0)
  (`HealthComponent.TakeDamage` (`/Game/core/blueprints/characters/player/BP_Player.Health Component` _asbp_player) 0))

(event `self.Request Object`
  (if (not (`self.Is Dead`))
    (`self.SetActorTickEnabled` true)
    (`|ExecutionSequence`
      (:`then_0`
        (`parent.Request Object`))
      (:`then_1`
        (bind (_direction _value) (`Timeline|Movement` :!via `PlayFromStart` :!label _label)
          (:`Update`
            (`SceneComponent.K2_SetRelativeLocation` (`self.CapsuleComponent`) (`|EaseFunction` "EaseInOut" _value (`self.Start Pos`) (`self.End Pos`)) false false))
          (:`Finished`
            (switch `ETimelineDirection` _direction
              (:`Forward`
                (`self.Reverse Timeline`))
              (:`Backward`
                (`self.Play Timeline`)))))))))

(event `Play Timeline`
  (goto _label :!via `PlayFromStart`))

(event `self.OnObjectDeactivated`
  (`parent.OnObjectDeactivated`)
  (`TimelineComponent.Stop` (`self.Movement`))
  (set `self.Is Dead` true)
  (`self.SetActorTickEnabled` false :!label _label_2))

(event `Reverse Timeline`
  (goto _label :!via `ReverseFromEnd`))

(event `self.On Death`
  (`parent.On Death`)
  (`TimelineComponent.Stop` (`self.Movement`))
  (set `self.Is Dead` true)
  (goto _label_2))

(fn `Get Laser End Position`
  (params (`Actor Position` :type "Vector Structure") (Forward :type "Vector Structure"))
  (returns (`End Position` :type "Vector Structure"))
  (return (+ `Actor Position` (* Forward (`self.Laser Distance`)))))

(fn `UserConstructionScript`
  (`parent.UserConstructionScript`))