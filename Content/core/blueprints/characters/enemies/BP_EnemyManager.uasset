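; BP_EnemyManager spawns an explosion wherever an explosive or chaser enemy despawns.
; On BeginPlay it binds one shared handler to the despawn event of every object in the explosive and chaser pools.
; That handler takes an object from the explosion pool and teleports it to the despawned object's location, so the effect reuses pooled actors.
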(event `self.ReceiveBeginPlay`
  (for _array_element (`/Game/core/blueprints/characters/enemies/BP_PawnPool.Objects` (`self.Explosive Pool`))
    (add `/Game/core/blueprints/characters/enemies/chaser/BP_PawnChaser.OnObjectDespawned` _array_element (delegate `Spawn Explosion`)))
  (for _array_element_2 (`/Game/core/blueprints/characters/enemies/BP_PawnPool.Objects` (`self.Chaser Pool`))
    (add `/Game/core/blueprints/characters/enemies/chaser/BP_PawnChaser.OnObjectDespawned` _array_element_2 (delegate `Spawn Explosion`))))

(event `Spawn Explosion`
  (params (Object :type "/Game/core/blueprints/characters/enemies/chaser/BP_PawnChaser Object Reference"))
  (bind _returnvalue (`ObjectPool.SpawnPooledObject` (`self.Explosion Pool`)))
  (`self.K2_SetActorLocation` _returnvalue (`self.K2_GetActorLocation` Object) false false))

(fn `UserConstructionScript`)