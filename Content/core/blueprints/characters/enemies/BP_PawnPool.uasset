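; BP_PawnPool is an object pool for enemy pawns that reuses instances instead of spawning on demand.
; Instantiate, optionally run at BeginPlay, pre-spawns inactive pawns at a distant location, indexes them and binds their despawn events.
; SpawnObject activates the first inactive pawn, or recycles the oldest active one via SpawnedIndexes when none are free.
; Despawning deactivates the pawn; BeginPlay also spawns and stores an AI controller.
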(event `Instantiate`
  (if (`KismetSystemLibrary.IsValidClass` (`self.Object Type`))
    (for _index (range (`self.Pool Size`))
      (bind _returnvalue (`|SpawnActorFromClass` (`self.Object Type`) (`KismetMathLibrary.MakeTransform` (0.0 20000.0 0.0)) "Undefined" "OverrideRootScale" null null))
      (`/Game/core/blueprints/characters/enemies/chaser/BP_PawnChaser.Set Active` _returnvalue false)
      (`/Game/core/blueprints/characters/enemies/chaser/BP_PawnChaser.Set Pool Index` _returnvalue _index)
      (`/Game/core/blueprints/characters/enemies/chaser/BP_PawnChaser.Deactivate` _returnvalue)
      (add `/Game/core/blueprints/characters/enemies/chaser/BP_PawnChaser.OnObjectDespawned` _returnvalue (delegate `On Object Despawn`))
      (`KismetArrayLibrary.Array_Add` (`self.Objects`) _returnvalue))))

(event `On Object Despawn`
  (params (Object :type "/Game/core/blueprints/characters/enemies/chaser/BP_PawnChaser Object Reference"))
  (`self.On Despawn` Object)
  (`KismetArrayLibrary.Array_RemoveItem` (`self.Spawned Indexes`) (`/Game/core/blueprints/characters/enemies/chaser/BP_PawnChaser.Pool Index` Object)))

(event `On Despawn`
  (params (Object :type "/Game/core/blueprints/characters/enemies/chaser/BP_PawnChaser Object Reference"))
  (`/Game/core/blueprints/characters/enemies/chaser/BP_PawnChaser.Set Active` Object false))

(event `self.ReceiveBeginPlay`
  (bind _returnvalue (`|SpawnActorFromClass` "/Script/AIModule.AIController" (`KismetMathLibrary.MakeTransform` (0.0 0.0 0.0)) "Undefined" "OverrideRootScale" null null))
  (set `self.Controller` _returnvalue)
  (if (`self.Spawn On Start`)
    (`self.Instantiate`)))

(fn `Setup Object`
  (params (Input :type "/Game/core/blueprints/characters/enemies/chaser/BP_PawnChaser Object Reference"))
  (`Actor.K2_SetActorTransform` Input (`KismetMathLibrary.MakeTransform` (0.0 0.0 0.0)) false false)
  (`/Game/core/blueprints/characters/enemies/chaser/BP_PawnChaser.Set Active` Input true)
  (`/Game/core/blueprints/characters/enemies/chaser/BP_PawnChaser.On Request` Input)
  (`KismetArrayLibrary.Array_Add` (`self.Spawned Indexes`) (`/Game/core/blueprints/characters/enemies/chaser/BP_PawnChaser.Pool Index` Input))
  (return))

(fn `Spawn Object`
  (returns (Output :type "/Game/core/blueprints/characters/enemies/chaser/BP_PawnChaser Object Reference"))
  (locals (`Pooled Object Index` :type Integer) (`Poolable Pawn` :type "/Game/core/blueprints/characters/enemies/chaser/BP_PawnChaser Object Reference"))
  (bind _spawned_indexes (`self.Spawned Indexes`))
  (for _array_element (`self.Objects`)
    (if (and (`KismetSystemLibrary.IsValid` _array_element) (not (`/Game/core/blueprints/characters/enemies/chaser/BP_PawnChaser.Active` _array_element)))
      (`self.Setup Object` _array_element)
      (return _array_element)))
  (if (> (`KismetArrayLibrary.Array_Length` (`self.Spawned Indexes`)) 0)
    (bind _output_get (set `local.Pooled Object Index` (`|GetArrayItem` _spawned_indexes)))
    (`KismetArrayLibrary.Array_RemoveItem` _spawned_indexes _output_get)
    (bind _output_get_2 (set `local.Poolable Pawn` (`|GetArrayItem` (`self.Objects`) (`local.Pooled Object Index`))))
    (`/Engine/EditorBlueprintResources/StandardMacros.IsValid` _output_get_2
      (:`Is Valid`
        (`/Game/core/blueprints/characters/enemies/chaser/BP_PawnChaser.Set Active` _output_get_2 true)
        (`self.Setup Object` _output_get_2)
        (return _output_get_2)))))