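; Pooled chaser enemy pawn that pursues the player and deals damage on capsule overlap.
; BeginPlay and RequestObject register it with the enemies subsystem and bind health events on first initialization.
; OnRequest plays a Niagara and timeline scale-in, then enables overlaps and starts AIMoveTo, reissued on each success.
; Death disables collision and movement, signals the kill and despawn, and unregisters the pawn.
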(event `self.ReceiveBeginPlay`
  (bind _health_component (`self.Health Component`))
  (`EnemiesSubsystem.AddPawn` (subsystem `EnemiesSubsystem`) self :!label _label)
  (`parent.ReceiveBeginPlay`)
  (`/Game/core/blueprints/utilities/BPML_Utilities.Is Enemy Pawn Initialized` self
    (:`False`
      (add `/Game/core/blueprints/generic/health-component/BP_EnemyHealthComponent.On Death` _health_component (delegate `On Death`))
      (add `/Game/core/blueprints/generic/health-component/BP_EnemyHealthComponent.On Damage Taken` _health_component (delegate `On Damage Taken`))
      (set `self.Init` true))))

(event `self.Capsule Component.OnComponentBeginOverlap`
  (params (OverlappedComponent :type "PrimitiveComponent Object Reference") (OtherActor :type "Actor Object Reference") (OtherComp :type "PrimitiveComponent Object Reference") (OtherBodyIndex :type Integer) (bFromSweep :type Boolean) (SweepResult :type "HitResult Structure (by ref)"))
  (bind _asbp_player (cast `/Game/core/blueprints/characters/player/BP_Player` OtherActor))
  (`HealthComponent.TakeDamage` (`/Game/core/blueprints/characters/player/BP_Player.Health Component` _asbp_player) 1))

(event `Request Object`
  (goto _label))

(event `On Death`
  (`self.Deactivate`)
  (`self.OnEnemyKilled`)
  (`EnemiesSubsystem.RemovePawn` (subsystem `EnemiesSubsystem`) self))

(event `On Damage Taken`)

(event `On Request`
  (`self.SetActorScale3D` (0.0 0.0 0.0))
  (`SceneComponent.SetVisibility` (`self.Niagara`) true false)
  (`KismetSystemLibrary.Delay` 0.2)
  (`PrimitiveComponent.SetCollisionEnabled` (`self.Capsule Component`) "QueryOnly")
  (bind (_direction _value) (`Timeline|Timeline_0`)
    (:`Update`
      (`self.SetActorScale3D` (`KismetMathLibrary.Conv_DoubleToVector` _value)))
    (:`Finished`
      (set `self.Enabled` true)
      (set `PrimitiveComponent.bGenerateOverlapEvents` true (`self.Capsule Component`))
      (`SceneComponent.SetVisibility` (`self.Niagara`) false false)
      (`|AIMoveTo` self (0.0 0.0 0.0) (`GameplayStatics.GetPlayerPawn` 0) 10.0 :!label _label_2
        (:`OnSuccess`
          (`self.Repeat`))))))

(event `On Disable`
  (bind _capsule_component (`self.Capsule Component`))
  (set `self.Enabled` false)
  (set `PrimitiveComponent.bGenerateOverlapEvents` false _capsule_component)
  (`PrimitiveComponent.SetCollisionEnabled` _capsule_component "NoCollision")
  (`self.OnObjectDespawned` self)
  (`NavMovementComponent.StopActiveMovement` (`self.FloatingPawnMovement`)))

(event `Repeat`
  (goto _label_2))

(fn `Activate`)

(fn `Deactivate`
  (`self.On Disable`))

(fn `Set Active`
  (params (Active :type Boolean))
  (set `self.Active` Active)
  (`self.SetActorHiddenInGame` (not Active)))

(fn `Set Pool Index`
  (params (Index :type Integer))
  (set `self.Pool Index` Index))

(fn `UserConstructionScript`)