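; BP_Chaser is an enemy that homes in on the player and deals damage on touch.
; BeginPlay caches the BP_Player actor, then Tick moves the chaser toward it with VInterpTo at MovementSpeed, without sweep, so it ignores blocking collision and slows as it nears.
; A capsule begin overlap with BP_Player calls TakeDamage on the player's HealthComponent.
; Death and damage-taken events defer to the parent class.
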(event `self.ReceiveBeginPlay`
  (`parent.ReceiveBeginPlay`)
  (bind _returnvalue (`GameplayStatics.GetActorOfClass` "/Game/core/blueprints/characters/player/BP_Player.BP_Player_C"))
  (set `self.Player` _returnvalue))

(event `self.ReceiveTick`
  (params (DeltaSeconds :type "Float (single-precision)"))
  (`self.K2_SetActorLocation` (`KismetMathLibrary.VInterpTo` (`self.K2_GetActorLocation`) (`self.K2_GetActorLocation` (`self.Player`)) (`GameplayStatics.GetWorldDeltaSeconds`) (`self.Movement Speed`))))

(event `self.On Death`
  (`parent.On Death`))

(event `self.On Damage Taken`
  (`parent.On Damage Taken`))

(event `self.CapsuleComponent.OnComponentBeginOverlap`
  (params (OverlappedComponent :type "PrimitiveComponent Object Reference") (OtherActor :type "Actor Object Reference") (OtherComp :type "PrimitiveComponent Object Reference") (OtherBodyIndex :type Integer) (bFromSweep :type Boolean) (SweepResult :type "HitResult Structure (by ref)"))
  (bind _asbp_player (cast `/Game/core/blueprints/characters/player/BP_Player` OtherActor))
  (`HealthComponent.TakeDamage` (`/Game/core/blueprints/characters/player/BP_Player.Health Component` _asbp_player)))

(fn `UserConstructionScript`
  (`parent.UserConstructionScript`))