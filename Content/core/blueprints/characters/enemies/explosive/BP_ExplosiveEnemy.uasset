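; Enemy Blueprint that explodes on death, damaging nearby actors.
; On death it runs the parent logic, sphere-overlaps within ExplosionRadius excluding itself, then calls TakeDamage on each valid HealthComponent found and prints a debug message.
; The construction script briefly draws a debug sphere to preview the blast radius.
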(event `self.On Death`
  (`parent.On Death`)
  (bind _outactors (`KismetSystemLibrary.SphereOverlapActors` (`self.K2_GetActorLocation`) (`self.Explosion Radius`) (`self.Object Types`) null (`|MakeArray` self :!type "Actor Object Reference")))
  (for _array_element _outactors
    (bind _returnvalue (`self.GetComponentByClass` _array_element "/Script/NexCore.HealthComponent"))
    (if (`KismetSystemLibrary.IsValid` _returnvalue)
      (`HealthComponent.TakeDamage` _returnvalue)
      (`KismetSystemLibrary.PrintString` (`KismetStringLibrary.Concat_StrStr` (`KismetSystemLibrary.GetDisplayName` _array_element) "  took damage!")))))

(fn `UserConstructionScript`
  (`parent.UserConstructionScript`)
  (`KismetSystemLibrary.DrawDebugSphere` (`self.K2_GetActorLocation`) (`self.Explosion Radius`) 12 (struct :`R` 1.0 :`G` 1.0 :`B` 1.0 :`A` 1.0) 0.1 3.0))