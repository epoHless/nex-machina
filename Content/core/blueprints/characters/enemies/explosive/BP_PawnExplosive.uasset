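; BP_PawnExplosive is an exploding enemy pawn that damages its surroundings when it dies.
; Its OnDeath event runs the parent death logic, then sphere-overlaps actors of set object types within ExplosionRadius of its location, ignoring itself.
; Each overlapped actor with a valid HealthComponent receives a TakeDamage call.
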(event `self.On Death`
  (`parent.On Death`)
  (bind _outactors (`KismetSystemLibrary.SphereOverlapActors` (`self.K2_GetActorLocation`) (`self.Explosion Radius`) (`self.Object Types`) null (`|MakeArray` self :!type "Actor Object Reference")))
  (for _array_element _outactors
    (bind _returnvalue (`self.GetComponentByClass` _array_element "/Script/NexCore.HealthComponent"))
    (if (`KismetSystemLibrary.IsValid` _returnvalue)
      (`HealthComponent.TakeDamage` _returnvalue))))

(fn `UserConstructionScript`
  (`parent.UserConstructionScript`))