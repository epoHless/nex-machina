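; BP_Boss is a boss enemy that shows its own health widget and drives a child-actor rotator when activated.
; Health thresholds switch patterns: at 70 a looping timer spawns pooled chasers at random points inside a box, up to a cap, while the third form at 30 is unimplemented.
; On death it stops spawning, deactivates the rotator and every pooled chaser, and spawns an explosion effect.
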(event `On Deactivate`
  (`KismetSystemLibrary.K2_PauseTimerHandle` (`self.Spawner Timer Handle`))
  (`/Game/core/blueprints/characters/enemies/boss/BP_Rotator.Deactivate` (`self.Rotator`))
  (for _array_element (`/Game/core/blueprints/characters/enemies/BP_PawnPool.Objects` (`/Game/core/blueprints/characters/enemies/BP_EnemyManager.Chaser Pool` (`self.Enemy Manager`)))
    (`/Game/core/blueprints/characters/enemies/chaser/BP_PawnChaser.Deactivate` _array_element))
  (`NiagaraFunctionLibrary.SpawnSystemAtLocation` "/Game/core/art/vfx/NS_BossExplosion.NS_BossExplosion" (+ (`self.K2_GetActorLocation`) (-150.0 0.0 0.0))))

(event `self.ReceiveBeginPlay`
  (bind _returnvalue (`|CreateWidget` "/Game/core/blueprints/UI/boss/WIDGET_Boss.WIDGET_Boss_C"))
  (bind _output_get (set `self.UI` _returnvalue))
  (set `/Game/core/blueprints/UI/boss/WIDGET_Boss.Boss` self _output_get)
  (add `/Game/core/blueprints/characters/enemies/boss/BP_BossHPComponent.On Boss Killed` (`self.Health Component`) (delegate `On Deactivate`)))

(event `Activate`
  (`UserWidget.AddToViewport` (`self.UI`) 0)
  (add `/Game/core/blueprints/characters/enemies/boss/BP_BossHPComponent.On Treshold Reached` (`self.Health Component`) (delegate `On Change Pattern`))
  (bind _asbp_rotator (cast `/Game/core/blueprints/characters/enemies/boss/BP_Rotator` (`ChildActorComponent.ChildActor` (`self.Rotator Actor`))))
  (bind _output_get (set `self.Rotator` _asbp_rotator))
  (`/Game/core/blueprints/characters/enemies/boss/BP_Rotator.Activate` _output_get))

(event `On Change Pattern`
  (params (Value :type Integer))
  (if (== Value 70)
    (bind _returnvalue (`KismetSystemLibrary.K2_SetTimerDelegate` (delegate `Spawn Enemy`) 0.5 true))
    (set `self.Spawner Timer Handle` _returnvalue)
    (else
      ;[1 1 1] Add third form
      (if (== Value 30)
        _))))

(event `Spawn Enemy`
  (bind (_returnvalue_x _returnvalue_y) (`KismetMathLibrary.BreakVector` (`self.Get Random Point`)))
  (bind _output (`/Game/core/blueprints/characters/enemies/BP_PawnPool.Spawn Object` (`/Game/core/blueprints/characters/enemies/BP_EnemyManager.Chaser Pool` (`self.Enemy Manager`))))
  (`self.K2_SetActorLocation` _output (`KismetMathLibrary.MakeVector` _returnvalue_x _returnvalue_y 90.0) false false)
  (bind _result (`/Engine/EditorBlueprintResources/StandardMacros.IncrementInt` (`self.Spawned Enemies`))
    (:`  `
      (if (>= _result 100)
        (`KismetSystemLibrary.K2_PauseTimerHandle` (`self.Spawner Timer Handle`))))))

(fn `Get Percentage Left`
  (returns (ReturnValue :type "Float (double-precision)"))
  (return (/ (`KismetMathLibrary.Conv_IntToDouble` (`HealthComponent.Health` (`self.Health Component`))) 100.0)))

(fn `Get Random Point`
  (returns (ReturnValue :type "Vector Structure"))
  (bind _box_spawner (`self.Box Spawner`))
  (return (`KismetMathLibrary.RandomPointInBoundingBox` (`SceneComponent.K2_GetComponentLocation` _box_spawner) (`BoxComponent.BoxExtent` _box_spawner))))

(fn `UserConstructionScript`)