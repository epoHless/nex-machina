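; BP_Rotator is a rotating boss turret that fires from four muzzles at a fixed rate.
; Activate starts a looping timer whose Shoot event reuses one child BP_EnemyShooter, looping over the muzzles to fire, then move it to that muzzle's transform and play a shot sound.
; Toggle pauses or resumes the timer, while Deactivate clears it and zeroes the rotation rate.
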(event `Activate`
  (set `self.Muzzles` (`|MakeArray` (`self.Muzzle_1`) (`self.Muzzle_2`) (`self.Muzzle_3`) (`self.Muzzle_4`)))
  (bind _asbp_enemy_shooter (cast `/Game/core/blueprints/generic/weapons/BP_EnemyShooter` (`ChildActorComponent.ChildActor` (`self.First Actor Shooter`))))
  (set `self.Shooter` _asbp_enemy_shooter)
  (bind _returnvalue (`KismetSystemLibrary.K2_SetTimerDelegate` (delegate `Shoot`) (`self.Fire Rate`) true))
  (set `self.Shooting Timer Handle` _returnvalue)
  (set `/Game/core/blueprints/generic/weapons/BP_Shooter.Fire Rate` (`self.Fire Rate`) (`self.Shooter`)))

(event `Shoot`
  (bind _shooter (`self.Shooter`))
  (for _array_element (`self.Muzzles`)
    (`/Game/core/blueprints/generic/weapons/BP_Shooter.Shoot` _shooter)
    (`self.K2_SetActorTransform` _shooter (`KismetMathLibrary.MakeTransform` (`SceneComponent.K2_GetComponentLocation` _array_element) (`SceneComponent.K2_GetComponentRotation` _array_element)) false false)
    (`GameplayStatics.PlaySoundAtLocation` "/Game/core/art/sounds/SFX_Turret_Shot.SFX_Turret_Shot" (`self.K2_GetActorLocation`) (struct) 1.0 1.0 0.0 "/Game/core/art/sounds/attenuation/NewSoundAttenuation_Turrets.NewSoundAttenuation_Turrets" null null null)))

(event `Deactivate`
  (`KismetSystemLibrary.K2_ClearAndInvalidateTimerHandle` (`self.Shooting Timer Handle`))
  (set `RotatingMovementComponent.RotationRate` (struct) (`self.RotatingMovement`)))

(fn `Toggle`
  (params (Toggle :type Boolean))
  (bind _shooting_timer_handle (`self.Shooting Timer Handle`))
  (if Toggle
    (`KismetSystemLibrary.K2_UnPauseTimerHandle` _shooting_timer_handle)
    (else
      (`KismetSystemLibrary.K2_PauseTimerHandle` _shooting_timer_handle))))

(fn `UserConstructionScript`)