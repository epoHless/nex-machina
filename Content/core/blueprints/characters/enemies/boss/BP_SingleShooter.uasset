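; BP_SingleShooter is a boss enemy Blueprint in the shooter family that extends a parent class.
; On Activate it runs the parent activation, then adds four muzzle components, Muzzle5 through Muzzle8, to the inherited Muzzles array.
; The construction script only calls the parent's version.
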(event `self.Activate`
  (`parent.Activate`)
  (`KismetArrayLibrary.Array_Add` (`self.Muzzles`) (`self.Muzzle_5`))
  (`KismetArrayLibrary.Array_Add` (`self.Muzzles`) (`self.Muzzle_6`))
  (`KismetArrayLibrary.Array_Add` (`self.Muzzles`) (`self.Muzzle_7`))
  (`KismetArrayLibrary.Array_Add` (`self.Muzzles`) (`self.Muzzle_8`)))

(fn `UserConstructionScript`
  (`parent.UserConstructionScript`))