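; Base enemy Blueprint that registers with the enemies subsystem and supports pool-style request and deactivation.
; BeginPlay and RequestObject share setup, deactivating unless EnableOnStart and binding HealthComponent death and damage events once.
; On request, a timeline animates actor scale before enabling the enemy and its overlaps, while deactivation switches both off along with collision.
; Death deactivates the enemy, broadcasts the kill and unregisters it; the damage handler is empty.
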(event `self.ReceiveBeginPlay`
  (bind _health_component (`self.Health Component`))
  (`EnemiesSubsystem.Add` (subsystem `EnemiesSubsystem`) self :!label _label)
  (if (not (`self.Enable On Start`))
    (`self.Deactivate`))
  (`parent.ReceiveBeginPlay`)
  (`/Game/core/blueprints/utilities/BPML_Utilities.Is Enemy Initialized` self
    (:`False`
      (add `/Game/core/blueprints/generic/health-component/BP_EnemyHealthComponent.On Death` _health_component (delegate `On Death`))
      (add `/Game/core/blueprints/generic/health-component/BP_EnemyHealthComponent.On Damage Taken` _health_component (delegate `On Damage Taken`))
      (set `self.Init` true))))

(event `Request Object`
  (goto _label))

(event `On Death`
  (`self.Deactivate`)
  (`self.OnEnemyKilled`)
  (`EnemiesSubsystem.Remove` (subsystem `EnemiesSubsystem`) self))

(event `On Damage Taken`)

(event `self.OnObjectRequest`
  (params (Direction :type "Vector Structure"))
  (`EnemiesSubsystem.Add` (subsystem `EnemiesSubsystem`) self)
  (`PrimitiveComponent.SetCollisionEnabled` (`self.CapsuleComponent`) "QueryOnly")
  (bind (_direction _value) (`Timeline|Scale`)
    (:`Update`
      (`self.SetActorScale3D` (`KismetMathLibrary.Conv_DoubleToVector` _value)))
    (:`Finished`
      (set `self.Enabled` true)
      (set `PrimitiveComponent.bGenerateOverlapEvents` true (`self.CapsuleComponent`)))))

(event `self.OnObjectDeactivated`
  (set `self.Enabled` false)
  (set `PrimitiveComponent.bGenerateOverlapEvents` false (`self.CapsuleComponent`))
  (`PrimitiveComponent.SetCollisionEnabled` (`self.CapsuleComponent`) "NoCollision"))

(fn `UserConstructionScript`)