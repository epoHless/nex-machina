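; GM_Standard is the game mode that opens play on a main menu and starts the level once Play is clicked.
; On BeginPlay it caches the level manager and player pawn, disables input and shows the WIDGET_MainMenu widget with its Play button bound.
; Clicking Play removes the menu, restores input in game-only mode, initializes the player's gun, then tells BP_LevelManager to start after a short delay.
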(event `self.ReceiveBeginPlay`
  (bind _returnvalue (`GameplayStatics.GetPlayerController` 0))
  (bind _returnvalue_2 (`GameplayStatics.GetActorOfClass` "/Game/core/blueprints/generic/level-management/BP_LevelManager.BP_LevelManager_C"))
  (set `self.Level Manager` _returnvalue_2)
  (bind _asbp_player (cast `/Game/core/blueprints/characters/player/BP_Player` (`GameplayStatics.GetPlayerPawn` 0)))
  (bind _output_get (set `self.Player` _asbp_player))
  (`self.DisableInput` _returnvalue _returnvalue)
  (`self.DisableInput` _output_get _returnvalue)
  (bind _returnvalue_3 (`|CreateWidget` "/Game/core/blueprints/UI/menu/WIDGET_MainMenu.WIDGET_MainMenu_C" (`GameplayStatics.GetPlayerController` 0)))
  (bind _output_get_2 (set `self.Main Menu UI` _returnvalue_3))
  (`UserWidget.AddToViewport` _output_get_2 1)
  (add `Button.OnClicked` (`/Game/core/blueprints/UI/custom-ui/menu-button/WID_BTN.btn` (`/Game/core/blueprints/UI/menu/WIDGET_MainMenu.btn_play` (`self.Main Menu UI`))) (delegate `On Clicked Play`)))

(event `On Clicked Play`
  (bind _returnvalue (`GameplayStatics.GetPlayerController` 0))
  (`Widget.RemoveFromParent` (`self.Main Menu UI`))
  (`self.EnableInput` _returnvalue _returnvalue)
  (`self.EnableInput` (`self.Player`) _returnvalue)
  (`/Game/core/blueprints/generic/weapons/BP_PlayerShooter.Initialize Weapon` (`/Game/core/blueprints/characters/player/BP_Player.Player Gun` (`self.Player`)))
  (`WidgetBlueprintLibrary.SetInputMode_GameOnly` _returnvalue)
  (`KismetSystemLibrary.Delay` 2.0)
  (`/Game/core/blueprints/generic/level-management/BP_LevelManager.Start Game` (`self.Level Manager`)))

(fn `UserConstructionScript`)